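; Police chief NPC that runs a three-part scripted conversation with the player, ending in an "Exit the Police Station" mission.
; It registers itself on the player character at BeginPlay, and each externally called chat event loads its own DataTable into BPCConversant and fades in Talking.
; Dialogue triggers fade Talking out, then show an interval widget after the first two chats or update the mission and re-enable player control after the last.
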(event `self.ReceiveBeginPlay`
  (`AudioComponent.FadeOut` (`self.Talking`) 0.0 0.0 "Linear")
  (bind _asbp_first_person_character (cast `/Game/FirstPerson/Blueprints/BP_FirstPersonCharacter` (`GameplayStatics.GetPlayerCharacter` 0)))
  (set `/Game/FirstPerson/Blueprints/BP_FirstPersonCharacter.CheifOfPolice` self _asbp_first_person_character))

(event `FirstChat`
  (bind _bpc_conversant (`self.BPC_Conversant`))
  ; The customers convo with the player in the diner to prove their innocence
  (set `/Game/DialogueSystem/BPC_Conversant.ConversationTabel` "/Game/DialogueSystem/DT_TalkingToDeputy.DT_TalkingToDeputy" _bpc_conversant)
  (set `/Game/DialogueSystem/BPC_Conversant.Name` "Cheif Cashew" _bpc_conversant)
  (add `/Game/DialogueSystem/BPC_Conversant.OnDialogueEventTrigger` _bpc_conversant (delegate `CustomEvent_2`))
  (`KismetSystemLibrary.Delay` 1.0)
  (`/Game/DialogueSystem/BPC_Conversant.StartConversation` (`self.BPC_Conversant`) "0")
  (`AudioComponent.FadeIn` (`self.Talking`) 0.0 1.0 0.0 "Linear"))

(event `CustomEvent_2`
  (params (`Dialogue Trigger` :type Name))
  ; The customers convo with the player in the diner to prove their innocence
  (if (== `Dialogue Trigger` "Interval")
    (`AudioComponent.FadeOut` (`self.Talking`) 0.0 0.0 "Linear")
    ; Interval
    (bind _returnvalue (`|CreateWidget` "/Game/DialogueSystem/WBP_DialogueInterval.WBP_DialogueInterval_C"))
    (bind _output_get (set `self.IntervalWidget` _returnvalue))
    (`UserWidget.AddToViewport` _output_get 0)
    (set `/Game/DialogueSystem/WBP_DialogueInterval.Policeman` self _output_get)))

(event `SecondChat`
  (bind _bpc_conversant (`self.BPC_Conversant`))
  ; Second Chat
  (`Widget.RemoveFromParent` (`self.IntervalWidget`))
  (set `/Game/DialogueSystem/BPC_Conversant.ConversationTabel` "/Game/DialogueSystem/DT_SecondChatToDeputy.DT_SecondChatToDeputy" _bpc_conversant)
  (set `/Game/DialogueSystem/BPC_Conversant.Name` "Cheif Cashew" _bpc_conversant)
  (add `/Game/DialogueSystem/BPC_Conversant.OnDialogueEventTrigger` _bpc_conversant (delegate `CustomEvent`))
  (`KismetSystemLibrary.Delay` 1.0)
  (`/Game/DialogueSystem/BPC_Conversant.StartConversation` (`self.BPC_Conversant`) "0")
  (`AudioComponent.FadeIn` (`self.Talking`) 0.0 1.0 0.0 "Linear"))

(event `CustomEvent`
  (params (`Dialogue Trigger` :type Name))
  ; Second Chat
  (if (== `Dialogue Trigger` "SecondInterval")
    (`AudioComponent.FadeOut` (`self.Talking`) 0.0 0.0 "Linear")
    ;; Second Interval
    (bind _returnvalue (`|CreateWidget` "/Game/DialogueSystem/WBP_DialogueInterval2.WBP_DialogueInterval2_C"))
    (bind _output_get (set `self.IntervalWidget2` _returnvalue))
    (`UserWidget.AddToViewport` _output_get 0)))

(event `ThirdChat`
  (bind _bpc_conversant (`self.BPC_Conversant`))
  ; Third/Last Chat
  (`Widget.RemoveFromParent` (`self.IntervalWidget2`))
  (set `/Game/DialogueSystem/BPC_Conversant.ConversationTabel` "/Game/DialogueSystem/DT_LastChatToDeputy.DT_LastChatToDeputy" _bpc_conversant)
  (set `/Game/DialogueSystem/BPC_Conversant.Name` "Cheif Cashew" _bpc_conversant)
  (add `/Game/DialogueSystem/BPC_Conversant.OnDialogueEventTrigger` _bpc_conversant (delegate `CustomEvent_3`))
  (`KismetSystemLibrary.Delay` 1.0)
  (`/Game/DialogueSystem/BPC_Conversant.StartConversation` (`self.BPC_Conversant`) "0")
  (`AudioComponent.FadeIn` (`self.Talking`) 0.0 1.0 0.0 "Linear"))

(event `CustomEvent_3`
  (params (`Dialogue Trigger` :type Name))
  ; Third/Last Chat
  (if (== `Dialogue Trigger` "DonutLadyDeathScene")
    (`AudioComponent.FadeOut` (`self.Talking`) 0.0 0.0 "Linear")
    (bind _asbp_first_person_character (cast `/Game/FirstPerson/Blueprints/BP_FirstPersonCharacter` (`GameplayStatics.GetPlayerCharacter` 0)))
    (`/Game/FirstPerson/Blueprints/BP_FirstPersonCharacter.UpdateMission` _asbp_first_person_character "Exit the Police Station" "")
    (`/Game/FirstPerson/Blueprints/BP_FirstPersonCharacter.Enable input + pawn rotation` _asbp_first_person_character)))

(fn `UserConstructionScript`)