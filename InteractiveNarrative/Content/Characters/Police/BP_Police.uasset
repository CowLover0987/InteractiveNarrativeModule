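; BP_Police is the police enemy that chases the player and catches them on contact.
; Pawn sensing sets a seen flag and starts an AI MoveTo toward the player, and a box overlap calls CaughtByPolice on the first-person character.
; It registers itself with the player at BeginPlay and stores its start location, so GoingBacktothebegining can teleport it back and show its mesh again.
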(event `self.ReceiveBeginPlay`
  ; Get starting location for respawning when the player is caught
  (set `self.BeginingLocation` (`self.K2_GetActorLocation`))
  (bind _asbp_first_person_character (cast `/Game/FirstPerson/Blueprints/BP_FirstPersonCharacter` (`GameplayStatics.GetPlayerCharacter` 0)))
  (set `/Game/FirstPerson/Blueprints/BP_FirstPersonCharacter.Police` self _asbp_first_person_character))

(event `self.PawnSensing.OnSeePawn`
  (params (Pawn :type "Pawn Object Reference"))
  ; 'Seeing' and following the player
  (set `self.IsSeeingPlayer` true)
  (`self.FollowPlayer`))

(event `Going Back to the begining`
  ; For returning to starting postion
  (`self.K2_SetActorLocation` (`self.BeginingLocation`))
  (`SceneComponent.SetVisibility` (`self.Mesh`) true false))

(event `FollowPlayer`
  ; 'Seeing' and following the player
  (if (`self.IsSeeingPlayer`)
    (`|AIMoveTo` self (0.0 0.0 0.0) (`GameplayStatics.GetPlayerCharacter` 0))))

(event `self.Box.OnComponentBeginOverlap`
  (params (OverlappedComponent :type "PrimitiveComponent Object Reference") (OtherActor :type "Actor Object Reference") (OtherComp :type "PrimitiveComponent Object Reference") (OtherBodyIndex :type Integer) (bFromSweep :type Boolean) (SweepResult :type "HitResult Structure (by ref)"))
  ; Detecting if player has been caught
  (bind _asbp_first_person_character (cast `/Game/FirstPerson/Blueprints/BP_FirstPersonCharacter` OtherActor))
  (`/Game/FirstPerson/Blueprints/BP_FirstPersonCharacter.CaughtByPolice` _asbp_first_person_character))

(fn `UserConstructionScript`)