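; Witness NPC Erica, who finds the player with the body and leads into the forest chase.
; On BeginPlay it configures its BPCConversant component with the DT_FindingTheBody table and starts the conversation after a short delay.
; A bound dialogue event listens for the "RunAway" trigger, which cuts the Talking audio and calls BeginForestChase on the first-person player character.
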(event `self.ReceiveBeginPlay`
  (bind _bpc_conversant (`self.BPC_Conversant`))
  ; Erica (Witness finding the player with the body)
  (set `/Game/DialogueSystem/BPC_Conversant.ConversationTabel` "/Game/DialogueSystem/DT_FindingTheBody.DT_FindingTheBody" _bpc_conversant)
  (set `/Game/DialogueSystem/BPC_Conversant.Name` "Erica" _bpc_conversant)
  (add `/Game/DialogueSystem/BPC_Conversant.OnDialogueEventTrigger` _bpc_conversant (delegate `CustomEvent_2`))
  (`KismetSystemLibrary.Delay` 1.0)
  (`/Game/DialogueSystem/BPC_Conversant.StartConversation` (`self.BPC_Conversant`) "0"))

(event `CustomEvent_2`
  (params (`Dialogue Trigger` :type Name))
  ; Erica (Witness finding the player with the body)
  (if (== `Dialogue Trigger` "RunAway")
    (`AudioComponent.FadeOut` (`self.Talking`) 0.0 0.0 "Linear")
    (bind _asbp_first_person_character (cast `/Game/FirstPerson/Blueprints/BP_FirstPersonCharacter` (`GameplayStatics.GetPlayerCharacter` 0)))
    (`/Game/FirstPerson/Blueprints/BP_FirstPersonCharacter.Begin Forest Chase` _asbp_first_person_character)))

(fn `UserConstructionScript`)