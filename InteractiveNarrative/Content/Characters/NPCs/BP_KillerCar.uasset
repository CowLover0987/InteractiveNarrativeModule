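; BP_KillerCar is an NPC car that drives toward a waypoint and ends the game if it hits the donut lady.
; On BeginPlay it grabs the first BP_Waypoint in the level, then after a short delay issues an AI MoveTo toward it.
; When its box overlaps BP_DonutLady, it pauses the game and shows the WBP_EndGame widget.
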(event `self.ReceiveBeginPlay`
  ; NPC following a waypoint set path
  (bind _returnvalue (`GameplayStatics.GetActorOfClass` "/Game/Characters/NPCs/BP_Waypoint.BP_Waypoint_C"))
  (set `self.Waypoint` _returnvalue)
  (`self.FollowWaypoints`))

(event `FollowWaypoints`
  ; NPC following a waypoint set path
  (`KismetSystemLibrary.Delay` 0.2)
  (`|AIMoveTo` self (0.0 0.0 0.0) (`self.Waypoint`)))

(event `self.Box.OnComponentBeginOverlap`
  (params (OverlappedComponent :type "PrimitiveComponent Object Reference") (OtherActor :type "Actor Object Reference") (OtherComp :type "PrimitiveComponent Object Reference") (OtherBodyIndex :type Integer) (bFromSweep :type Boolean) (SweepResult :type "HitResult Structure (by ref)"))
  (cast `/Game/Characters/NPCs/DonutLady/BP_DonutLady` OtherActor)
  (`GameplayStatics.SetGamePaused` true)
  (bind _returnvalue (`|CreateWidget` "/Game/ObjectiveSyste/WBP_EndGame.WBP_EndGame_C"))
  (`UserWidget.AddToViewport` _returnvalue 0))

(fn `UserConstructionScript`)