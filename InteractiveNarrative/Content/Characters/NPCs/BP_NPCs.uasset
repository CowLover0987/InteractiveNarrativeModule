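; BP_NPCs is an NPC that patrols a looping set of waypoints.
; On BeginPlay, FollowWaypoints sends the pawn to the current waypoint with AIMoveTo.
; On success it advances the index, wrapping to the first after the last, waits briefly, then calls itself again.
; A failed move has no handler, so it ends the patrol.
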(event `self.ReceiveBeginPlay`
  ; NPC following a waypoint set path
  (`self.FollowWaypoints`))

(event `FollowWaypoints`
  ; NPC following a waypoint set path
  (`|AIMoveTo` self (0.0 0.0 0.0) (`|GetArrayItem` (`self.Waypoints`) (`self.CurrentWaypoint`))
    (:`OnSuccess`
      (`/Engine/EditorBlueprintResources/StandardMacros.IncrementInt` (`self.CurrentWaypoint`)
        (:`  `
          (if (>= (`self.CurrentWaypoint`) (`KismetArrayLibrary.Array_Length` (`self.Waypoints`)))
            (set `self.CurrentWaypoint` 0))
          (`KismetSystemLibrary.Delay` 3.0)
          (`self.FollowWaypoints`))))))

(fn `UserConstructionScript`)