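; Actor component that runs the UI side of a dialogue conversation and relays dialogue triggers to other Blueprints.
; StartConversation creates the WBP_ConvMain widget from a first row name, passing itself in, then switches to UI-only input with the cursor shown.
; A DoOnce blocks repeat starts until EndConversation removes the widget and restores game input.
; DialogueTrigger rebroadcasts any trigger name other than None through the OnDialogueEventTrigger dispatcher.
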(event `StartConversation`
  (params (FirstRowName :type Name))
  (bind _returnvalue (`GameplayStatics.GetPlayerController` 0))
  ; Start conversation (open widget and change input mode to UI)
  (`/Engine/EditorBlueprintResources/StandardMacros.DoOnce` false :!label _label
    (:`Completed`
      (bind _returnvalue_2 (`|CreateWidget` "/Game/DialogueSystem/WBP_ConvMain.WBP_ConvMain_C" null FirstRowName self))
      (bind _output_get (set `self.ConversationWidget` _returnvalue_2))
      (`UserWidget.AddToViewport` _output_get 0)
      (`WidgetBlueprintLibrary.SetInputMode_UIOnlyEx` _returnvalue _output_get)
      (set `PlayerController.bShowMouseCursor` true _returnvalue))))

(event `EndConversation`
  (bind _returnvalue (`GameplayStatics.GetPlayerController` 0))
  ; End conversation (close widget and return to game mode)
  (`Widget.RemoveFromParent` (`self.ConversationWidget`))
  (set `PlayerController.bShowMouseCursor` false _returnvalue)
  (`WidgetBlueprintLibrary.SetInputMode_GameOnly` _returnvalue)
  (set `self.ConversationWidget` null)
  (goto _label :!via `Reset`))

(event `DialogueTrigger`
  (params (TriggerName :type Name))
  ; Dialogue Event Trigger
  (if (!= TriggerName "None")
    (`self.OnDialogueEventTrigger` TriggerName)))