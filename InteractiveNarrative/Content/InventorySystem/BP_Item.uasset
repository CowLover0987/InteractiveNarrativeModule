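; BP_Item is a pickup actor for the inventory system, with a widget shown while anything overlaps its LabelTrigger.
; On BeginPlay it writes itself into the first-person character's Item variable, so each new instance overwrites that reference.
; PickUpItem prints a message, triggers a briefly delayed destroy and returns its Item.
; SpawningItem spawns another BP_Item at a location, but sets Item on itself rather than the spawned actor.
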(event `self.ReceiveBeginPlay`
  ; Setting varible in player character
  (bind _asbp_first_person_character (cast `/Game/FirstPerson/Blueprints/BP_FirstPersonCharacter` (`GameplayStatics.GetPlayerCharacter` 0)))
  (set `/Game/FirstPerson/Blueprints/BP_FirstPersonCharacter.Item` self _asbp_first_person_character))

(event `Destroy Item`
  ; Destroys item after being picked up
  (`KismetSystemLibrary.Delay` 0.1)
  (`self.K2_DestroyActor`))

(event `self.LabelTrigger.OnComponentBeginOverlap`
  (params (OverlappedComponent :type "PrimitiveComponent Object Reference") (OtherActor :type "Actor Object Reference") (OtherComp :type "PrimitiveComponent Object Reference") (OtherBodyIndex :type Integer) (bFromSweep :type Boolean) (SweepResult :type "HitResult Structure (by ref)"))
  ; Make widget visible indicating item can be picked up
  (`SceneComponent.SetVisibility` (`self.PickUp Widget`) true false))

(event `self.LabelTrigger.OnComponentEndOverlap`
  (params (OverlappedComponent :type "PrimitiveComponent Object Reference") (OtherActor :type "Actor Object Reference") (OtherComp :type "PrimitiveComponent Object Reference") (OtherBodyIndex :type Integer))
  ; Make widget visible indicating item can be picked up
  (`SceneComponent.SetVisibility` (`self.PickUp Widget`) false false))

(event `Spawning Item`
  (params (Item :type String) (SpawningLocation :type "Vector Structure"))
  ; Spawning actor
  (`|SpawnActorFromClass` "BP_Item_C" (`KismetMathLibrary.MakeTransform` SpawningLocation) "Undefined" "MultiplyWithRoot" null null)
  (set `self.Item` Item))

(fn `Pick Up Item`
  (returns (Item :type String))
  (`KismetSystemLibrary.PrintString` "Item picked up")
  (`self.Destroy Item`)
  (return (`self.Item`)))

(fn `UserConstructionScript`)